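; AC_Inventory is an inventory component that lets the player pick up items and stack them by name.
; On IA_PickUp completion, a debug-drawn sphere trace runs forward from the connected actor's first-person camera.
; A hit A_MasterPickUpItem supplies item data to a name-keyed map, either as a new entry or by incrementing the existing Amount by one.
; A successful add prints a message and destroys the world actor.
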(event `EnhancedInput|/Game/Inventory/Blueprints/IA_PickUp`
  (params (ActionValue :type Boolean) (ElapsedSeconds :type "Float (double-precision)") (TriggeredSeconds :type "Float (double-precision)") (InputAction :type "InputAction Object Reference" :default "/Game/Inventory/Blueprints/IA_PickUp.IA_PickUp"))
  (bind _firstpersoncamera (`/Game/FirstPerson/Blueprints/BP_FirstPersonCharacter.FirstPersonCamera` (`self.ConnectedActor`)))
  (bind _returnvalue (`SceneComponent.K2_GetComponentLocation` _firstpersoncamera))
  ;[1 1 1] Направление камеры
  (:`Completed`
    (bind (_outhit _returnvalue_2) (`KismetSystemLibrary.SphereTraceSingle` :`Start` _returnvalue :`End` (+ _returnvalue (* (`SceneComponent.GetForwardVector` _firstpersoncamera) 500)) :`Radius` 10.0 :`TraceChannel` "TraceTypeQuery1" :`DrawDebugType` "ForDuration"))
    (if _returnvalue_2
      (bind (_bblockinghit _binitialoverlap _time _distance _location _impactpoint _normal _impactnormal _physmat _hitactor) (`GameplayStatics.BreakHitResult` _outhit))
      (bind _added_ (`self.TryAddItem` _hitactor))
      (if _added_
        (`Actor.K2_DestroyActor` _hitactor)))))

(fn `Add Item to Inventary`
  (params (Item :type "/Game/Inventory/Blueprints/S_ItemData Structure"))
  (`BlueprintMapLibrary.Map_Add` (`self.Inventory`) (`.Name_12_0B1CBD414542BBA3886AFB9B83C55DC7` (break `/Game/Inventory/Blueprints/S_ItemData` Item)) Item))

(fn `IncreaseItemAmount`
  (params (Item :type "/Game/Inventory/Blueprints/S_ItemData Structure"))
  (locals (ItemName :type String))
  (bind _value (`BlueprintMapLibrary.Map_Find` (`self.Inventory`) (`local.ItemName`)))
  (set `local.ItemName` (`.Name_12_0B1CBD414542BBA3886AFB9B83C55DC7` (break `/Game/Inventory/Blueprints/S_ItemData` Item)))
  (bind _result (`/Engine/EditorBlueprintResources/StandardMacros.IncrementInt` (`.Amount_15_78BDD6344ADE9F8732B38E8091AD1E50` (break `/Game/Inventory/Blueprints/S_ItemData` _value)))
    (:`  `
      (bind _structout (setmembers `/Game/Inventory/Blueprints/S_ItemData` :`StructRef` _value :`Amount` _result))
      (`BlueprintMapLibrary.Map_Add` (`self.Inventory`) (`local.ItemName`) _structout))))

(fn `IsItemAlreadyInInventory`
  (params (Item :type "/Game/Inventory/Blueprints/S_ItemData Structure"))
  (returns (ReturnValue :type Boolean))
  (return (`BlueprintMapLibrary.Map_Contains` (`self.Inventory`) (`.Name_12_0B1CBD414542BBA3886AFB9B83C55DC7` (break `/Game/Inventory/Blueprints/S_ItemData` Item)))))

(fn `TryAddItem`
  (params (HitActor :type "Actor Object Reference"))
  (returns (`Added?` :type Boolean))
  (locals (CurrentItem :type "/Game/Inventory/Blueprints/S_ItemData Structure"))
  (bind _currentitem (`local.CurrentItem`))
  (bind _asa_master_pick_up_item (cast `/Game/Inventory/Blueprints/A_MasterPickUpItem` HitActor)
    (:`then`
      (bind _output_get (set `local.CurrentItem` (`/Game/Inventory/Blueprints/A_MasterPickUpItem.GetItemData` _asa_master_pick_up_item)))
      (if (`self.IsItemAlreadyInInventory` _output_get)
        (`self.IncreaseItemAmount` _currentitem)
        (else
          (`self.Add Item to Inventary` _currentitem)))
      (`KismetSystemLibrary.PrintString` (`KismetStringLibrary.Concat_StrStr` (`.Name_12_0B1CBD414542BBA3886AFB9B83C55DC7` (break `/Game/Inventory/Blueprints/S_ItemData` _currentitem)) "Added"))
      (return true))
    (:`CastFailed`
      (set `local.CurrentItem` (struct))
      (return false))))