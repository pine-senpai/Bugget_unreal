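; Blueprint for an animated 3D printer with an openable front window that produces a top cover actor.
; OpenDoor toggles the window's yaw through a timeline, but only while no print is in process.
; CallPrint chains timelines that move the supply, knot and fixation meshes, repeats a loop timeline via a counter, then plays a closing timeline in reverse.
; When that finishes, it clears InProcess and spawns the cover beside the printer, guarded by DoOnce.
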(event `self.ReceiveBeginPlay`)

(event `self.Open_door`
  (if (not (`self.InProcess`))
    (`/Engine/EditorBlueprintResources/StandardMacros.FlipFlop`
      (:`A`
        (bind (_direction _newtrack_0) (`Timeline|Timeline` :!via `PlayFromStart` :!label _label)
          (:`Update`
            (`SceneComponent.K2_SetRelativeRotation` (`self.MyPrinter3D_window_front_001`) (`KismetMathLibrary.MakeRotator` 0.0 0.0 _newtrack_0) false false))))
      (:`B`
        (goto _label :!via `ReverseFromEnd`)))))

(event `StartNewLoop`
  (bind (_direction _supply _down) (`Timeline|loop` :!via `PlayFromStart`)
    (:`Update`
      (`SceneComponent.K2_SetRelativeLocation` (`self.MyPrinter3D_fixation_supply_001`) (`KismetMathLibrary.MakeVector` 0.0 _supply) false false)
      (`SceneComponent.K2_SetRelativeLocation` (`self.MyPrinter3D_fixation_009`) (`KismetMathLibrary.MakeVector` _down) false false))
    (:`Finished`
      (if (< (`self.count`) 10)
        (bind _result (`/Engine/EditorBlueprintResources/StandardMacros.IncrementInt` (`self.count`))
          (:`  `
            (set `self.count` _result)
            (`self.StartNewLoop`)))
        (else
          (set `self.count` 0)
          (bind (_direction_2 _supply_2 _height _down_2) (`Timeline|Шкала времени_1` :!via `ReverseFromEnd`)
            (:`Update`
              (`SceneComponent.K2_SetRelativeLocation` (`self.MyPrinter3D_fixation_supply_001`) (`KismetMathLibrary.MakeVector` 0.0 _supply_2) false false)
              (`SceneComponent.K2_SetRelativeLocation` (`self.MyPrinter3D_fixation_knot_001`) (`KismetMathLibrary.MakeVector` 0.0 0.0 _height) false false)
              (`SceneComponent.K2_SetRelativeLocation` (`self.MyPrinter3D_fixation_009`) (`KismetMathLibrary.MakeVector` _down_2) false false))
            (:`Finished`
              (set `self.InProcess` false)
              (`/Engine/EditorBlueprintResources/StandardMacros.DoOnce` false
                (:`Completed`
                  (`|SpawnActorFromClass` "/Game/Inventory/Actor_Drone/A_D_TopCover.A_D_TopCover_C" (`KismetMathLibrary.MakeTransform` (+ (`SceneComponent.GetSocketLocation` (`self.DefaultSceneRoot`) "None") (0.0 -100.0 50.0)) (struct) (0.5 0.5 0.5)) "Undefined" "MultiplyWithRoot" null null))))))))))

(event `self.call_print`
  (set `self.InProcess` true)
  (bind (_direction _supply _height _down) (`Timeline|printing_start` :!via `PlayFromStart`)
    (:`Update`
      (`SceneComponent.K2_SetRelativeLocation` (`self.MyPrinter3D_fixation_supply_001`) (`KismetMathLibrary.MakeVector` 0.0 _supply) false false)
      (`SceneComponent.K2_SetRelativeLocation` (`self.MyPrinter3D_fixation_knot_001`) (`KismetMathLibrary.MakeVector` 0.0 0.0 _height) false false)
      (`SceneComponent.K2_SetRelativeLocation` (`self.MyPrinter3D_fixation_009`) (`KismetMathLibrary.MakeVector` _down) false false))
    (:`Finished`
      (bind (_direction_2 _supply_2 _down_2) (`Timeline|Шкала времени`)
        (:`Update`
          (`SceneComponent.K2_SetRelativeLocation` (`self.MyPrinter3D_fixation_supply_001`) (`KismetMathLibrary.MakeVector` 0.0 _supply_2) false false)
          (`SceneComponent.K2_SetRelativeLocation` (`self.MyPrinter3D_fixation_009`) (`KismetMathLibrary.MakeVector` _down_2) false false))
        (:`Finished`
          (`self.StartNewLoop`))))))

(fn `UserConstructionScript`)